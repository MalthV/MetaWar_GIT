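; BP_Cover is a cover-spot actor that tracks whether a BP_BlueDummy is within range to take cover.
; Its Box overlap begin and end events filter for that class, set a CanTakeCover flag true or false, then pass it to a CanTakeCover call.
; The CanTakeCover? and IsEnemy functions are stubs, with IsEnemy returning a zero vector.
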(event `self.Box.OnComponentBeginOverlap`
  (params (OverlappedComponent :type "PrimitiveComponent Object Reference") (OtherActor :type "Actor Object Reference") (OtherComp :type "PrimitiveComponent Object Reference") (OtherBodyIndex :type Integer) (bFromSweep :type Boolean) (SweepResult :type "HitResult Structure (by ref)"))
  (cast `/Game/Units/Dummy/Blue_Dummy/BP_BlueDummy` OtherActor)
  (bind _output_get (set `self.CanTakeCover` true))
  (`self.CanTakeCover?` _output_get))

(event `self.Box.OnComponentEndOverlap`
  (params (OverlappedComponent :type "PrimitiveComponent Object Reference") (OtherActor :type "Actor Object Reference") (OtherComp :type "PrimitiveComponent Object Reference") (OtherBodyIndex :type Integer))
  (cast `/Game/Units/Dummy/Blue_Dummy/BP_BlueDummy` OtherActor)
  (bind _output_get (set `self.CanTakeCover` false))
  (`self.CanTakeCover?` _output_get))

(fn `CanTakeCover?`
  (params (CanTakeCover :type Boolean))
  (return))

(fn `IsEnemy`
  (params (IsEnemy :type Boolean) (EnemyLocation :type "Vector Structure"))
  (returns (ELocation :type "Vector Structure"))
  (return (0.0 0.0 0.0)))

(fn `UserConstructionScript`)