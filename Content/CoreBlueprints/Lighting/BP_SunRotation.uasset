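; BP_SunRotation rotates a referenced sun actor to follow game time in an RTS.
; On BeginPlay it reads the game speed from BP_RTSGameState and binds an event that keeps that speed updated.
; Each tick, SetGameTime turns delta time and game speed into a time value, which is scaled into a local pitch rotation on the sun.
; The sky sphere's sun-direction update is disconnected, noted as a buggy reference.
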(event `self.ReceiveBeginPlay`
  (set `self.RTSGame State REF` (cast `/Game/CoreBlueprints/BP_RTSGameState` (`GameplayStatics.GetGameState`) :!pure true))
  (add `/Game/CoreBlueprints/BP_RTSGameState.GameSpeedControll` (`self.RTSGame State REF`) (`|CreateDelegate` :!event `GetGameSpeed`))
  (bind _gamespeed (`/Game/CoreBlueprints/BP_RTSGameState.GetGameSpeed` (`self.RTSGame State REF`)))
  (set `self.Game Speed` _gamespeed))

(event `GetGameSpeed`
  (params (GameSpeed :type "Float (double-precision)"))
  (set `self.Game Speed` GameSpeed))

(event `self.ReceiveTick`
  (params (DeltaSeconds :type "Float (single-precision)"))
  (`self.K2_AddActorLocalRotation` (`self.SunRef`) (`KismetMathLibrary.MakeRotator` 0.0 (* (/ (/ (`/Game/CoreBlueprints/Library/FunctionLibrary_RTS.Set Game Time` DeltaSeconds (`self.Game Speed`) (`self.GameTime`)) 1.5) 6.0) 90.0)) false false))

(fn `UserConstructionScript`)