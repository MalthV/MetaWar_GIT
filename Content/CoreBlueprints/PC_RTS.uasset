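; PC_RTS is an RTS player controller that drives the BP_CameraPawn camera, cached on BeginPlay alongside Game-and-UI input with a locked mouse.
; Axis inputs move the pawn relative to its facing with sweep, and zoom actions adjust or reset spring arm length within limits.
; Holding Pan opens a gate so MouseX yaws the pawn, with a separate yaw reset.
; A MouseEdgeMovement macro computes edge scrolling, but its calling logic is disconnected.
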(event `self.ReceiveTick`
  (params (DeltaSeconds :type "Float (single-precision)"))
  (set `self.Delta Seconds` DeltaSeconds))

(event `self.ReceiveBeginPlay`
  (`|ExecutionSequence`
    (:`then_0`
      (`self.Reference Cast`))
    (:`then_1`
      (`WidgetBlueprintLibrary.SetInputMode_GameAndUIEx` self null "LockAlways" false))))

(event `InputAxis|MoveForward`
  (params (AxisValue :type "Float (single-precision)"))
  (bind _camerapawnref (`self.CameraPawnRef`))
  (bind _returnvalue (`self.GetTransform` _camerapawnref))
  ;[1 1 1] Camera Movement
  (`self.K2_SetActorLocation` _camerapawnref (+ (`KismetMathLibrary.TransformDirection` _returnvalue (`KismetMathLibrary.MakeVector` (* (* AxisValue (`self.CameraMoveSpeed`)) (`self.MovementSpeedModifier`)))) (.location _returnvalue)) true false))

(event `InputAxis|MoveSideWays`
  (params (AxisValue :type "Float (single-precision)"))
  (bind _camerapawnref (`self.CameraPawnRef`))
  (bind _returnvalue (`self.GetTransform` _camerapawnref))
  ;[1 1 1] Camera Movement
  (`self.K2_SetActorLocation` _camerapawnref (+ (`KismetMathLibrary.TransformDirection` _returnvalue (`KismetMathLibrary.MakeVector` 0.0 (* (* AxisValue (`self.CameraMoveSpeed`)) (`self.MovementSpeedModifier`)))) (.location _returnvalue)) true false))

(event `InputAction|Zoom Reset`
  (params (Key :type "Key Structure"))
  ;[1 1 1] Reset Zoom
  (:`Pressed`
    (set `SpringArmComponent.TargetArmLength` 1300.0 (`/Game/CoreBlueprints/BP_CameraPawn.SpringArm` (`self.CameraPawnRef`)))))

(event `InputAction|ZoomIn`
  (params (Key :type "Key Structure"))
  (bind _springarm (`/Game/CoreBlueprints/BP_CameraPawn.SpringArm` (`self.CameraPawnRef`)))
  ;[1 1 1] Zoom In && Zoom Out Controll
  (:`Pressed`
    (set `SpringArmComponent.TargetArmLength` (`KismetMathLibrary.FClamp` (- (`SpringArmComponent.TargetArmLength` _springarm) (`self.ZoomSpeed`)) (`self.ZoomLimit_Min`) (`self.ZoomLimit_Max`)) _springarm)))

(event `InputAction|ZoomOut`
  (params (Key :type "Key Structure"))
  (bind _springarm (`/Game/CoreBlueprints/BP_CameraPawn.SpringArm` (`self.CameraPawnRef`)))
  ;[1 1 1] Zoom In && Zoom Out Controll
  (:`Pressed`
    (set `SpringArmComponent.TargetArmLength` (`KismetMathLibrary.FClamp` (+ (`SpringArmComponent.TargetArmLength` _springarm) (`self.ZoomSpeed`)) (`self.ZoomLimit_Min`) (`self.ZoomLimit_Max`)) _springarm)))

(event `InputAction|Pan`
  (params (Key :type "Key Structure"))
  (bind _camerapawnref (`self.CameraPawnRef`))
  (bind (_returnvalue_roll _returnvalue_pitch _returnvalue_yaw) (`KismetMathLibrary.BreakRotator` (`self.K2_GetActorRotation` _camerapawnref)))
  ;[1 1 1] PAN
  (:`Pressed`
    (set `self.IsPanning` true)
    (goto _label :!via `Open`))
  (:`Released`
    (set `self.IsPanning` false)
    (goto _label :!via `Close`)))

(event `InputAxisKey|MouseX`
  (params (AxisValue :type "Float (single-precision)"))
  (bind _camerapawnref (`self.CameraPawnRef`))
  (bind (_returnvalue_roll _returnvalue_pitch _returnvalue_yaw) (`KismetMathLibrary.BreakRotator` (`self.K2_GetActorRotation` _camerapawnref)))
  ;[1 1 1] PAN
  (`/Engine/EditorBlueprintResources/StandardMacros.Gate` true :!label _label
    (:`Exit`
      (`self.K2_SetActorRotation` _camerapawnref (`KismetMathLibrary.MakeRotator` _returnvalue_roll _returnvalue_pitch (+ _returnvalue_yaw (* AxisValue (`self.Pan Speed`)))) false))))

(event `InputAction|Pan Reset`
  (params (Key :type "Key Structure"))
  (bind _camerapawnref (`self.CameraPawnRef`))
  (bind (_returnvalue_roll _returnvalue_pitch) (`KismetMathLibrary.BreakRotator` (`self.K2_GetActorRotation` _camerapawnref)))
  ;[1 1 1] PAN Reset
  (:`Pressed`
    (`self.K2_SetActorRotation` _camerapawnref (`KismetMathLibrary.MakeRotator` _returnvalue_roll _returnvalue_pitch) false)))

(event `InputAxisKey|MouseX`
  (params (AxisValue :type "Float (single-precision)")))

(event `InputAxisKey|MouseY`
  (params (AxisValue :type "Float (single-precision)")))

(fn `UserConstructionScript`)